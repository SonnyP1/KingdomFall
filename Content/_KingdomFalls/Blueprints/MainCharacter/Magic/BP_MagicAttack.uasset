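; Magic attack projectile that homes in on a target for about a second, then flies straight until its timeline ends and destroys it.
; StartMoving runs the timeline, pushing it forward a fixed step per update while facing a target location that DelayLoc's self-calling delay loop refreshes periodically.
; Overlapping the assigned target calls TookDmg on a BaseAI or Hit on a KingdomFalls character, then destroys the projectile.
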(event `StopTracking`
  (`KismetSystemLibrary.Delay` 1.0)
  (set `self.isStopTracking` true))

(event `StartMoving`
  (`self.StopTracking`)
  (`self.DelayLoc`)
  (`Timeline|Lerping`
    (:`Update`
      (`/Engine/EditorBlueprintResources/StandardMacros.IsValid` (`self.TargetToAttack`)
        (:`Is Valid`
          (if (not (`self.isStopTracking`))
            (`self.K2_SetActorRotation` (`KismetMathLibrary.FindLookAtRotation` (`self.K2_GetActorLocation`) (`self.TargetLoc`)))))
        (:`Is Not Valid`
          _))
      (`self.K2_AddActorLocalOffset` (20.0 0.0 0.0)))
    (:`Finished`
      (`self.K2_DestroyActor`))))

(event `DelayLoc`
  (bind _targettoattack (`self.TargetToAttack`))
  (`/Engine/EditorBlueprintResources/StandardMacros.IsValid` _targettoattack
    (:`Is Valid`
      (set `self.TargetLoc` (`self.K2_GetActorLocation` _targettoattack))
      (`KismetSystemLibrary.Delay` 0.1)
      (if (not (`self.isStopTracking`))
        (`self.DelayLoc`)))
    (:`Is Not Valid`
      (`KismetSystemLibrary.PrintString` "Not Valid"))))

(event `self.ReceiveActorBeginOverlap`
  (params (OtherActor :type "Actor Object Reference"))
  (bind _targettoattack (`self.TargetToAttack`))
  (`KismetSystemLibrary.PrintString` "Hello")
  (if (== (`self.TargetToAttack`) OtherActor)
    (bind _asbase_ai (cast `/Game/_KingdomFalls/Blueprints/AI/BaseAI` _targettoattack)
      (:`then`
        (`/Game/_KingdomFalls/Blueprints/AI/BaseAI.Took Dmg` _asbase_ai 100.0)
        (`self.K2_DestroyActor`))
      (:`CastFailed`
        (bind _asbp_kingdom_falls_character (cast `/Game/_KingdomFalls/Blueprints/MainCharacter/BP_KingdomFallsCharacter` _targettoattack))
        (`/Game/_KingdomFalls/Blueprints/MainCharacter/BP_KingdomFallsCharacter.Hit` _asbp_kingdom_falls_character self)
        (`self.K2_DestroyActor`)))))

(fn `UserConstructionScript`)