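; GA_HitStun is a gameplay ability that resolves a hit on a Kingdom Falls character as either a block or damage taken.
; On activation, a blocking character calls Block if its forward vector opposes the attacker's, judged by a negative dot product.
; Otherwise it commits the ability cost and calls TookDmg.
; The ability ends immediately after either branch, leaving any reaction to the character's own functions.
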(event `self.K2_ActivateAbility`
  (bind _returnvalue_owneractor (break `GameplayAbilityActorInfo` (`self.GetActorInfo`)))
  (bind _asbp_kingdom_falls_character (cast `/Game/_KingdomFalls/Blueprints/MainCharacter/BP_KingdomFallsCharacter` _returnvalue_owneractor))
  (if (`/Game/_KingdomFalls/Blueprints/MainCharacter/BP_KingdomFallsCharacter.isBlocking` _asbp_kingdom_falls_character)
    (if (< (`KismetMathLibrary.Dot_VectorVector` (`Actor.GetActorForwardVector` _asbp_kingdom_falls_character) (`Actor.GetActorForwardVector` (`/Game/_KingdomFalls/Blueprints/MainCharacter/BP_KingdomFallsCharacter.Attacker` _asbp_kingdom_falls_character))) 0.0)
      (`/Game/_KingdomFalls/Blueprints/MainCharacter/BP_KingdomFallsCharacter.Block` _asbp_kingdom_falls_character)
      (else
        (`self.K2_CommitAbilityCost` false :!label _label)
        (`/Game/_KingdomFalls/Blueprints/MainCharacter/BP_KingdomFallsCharacter.TookDmg` _asbp_kingdom_falls_character)))
    (else
      (goto _label)))
  (`self.K2_EndAbility`))