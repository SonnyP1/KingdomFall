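; GA_StaminaRegen is a Gameplay Ability for the main character that regenerates stamina over time.
; On activation it waits through an initial delay, then compares two ability system attributes, presumably current and maximum stamina.
; Until the first reaches the second, it applies GE_RegenStamina to itself and repeats through a short WaitDelay loop, then ends the ability.
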(event `RegenAgain`
  (`AbilityTask_WaitDelay.WaitDelay` 0.1
    (:`OnFinish`
      (`self.RegenStaminaFunction` false :!label _label))))

(event `self.K2_ActivateAbility`
  (`AbilityTask_WaitDelay.WaitDelay` 2.0
    (:`OnFinish`
      (goto _label))))

(event `self.K2_OnEndAbility`
  (params (bWasCancelled :type Boolean)))

(fn `RegenStaminaFunction`
  (params (WasCancel :type Boolean))
  (bind (_returnvalue_owneractor _returnvalue_avataractor _returnvalue_playercontroller _returnvalue_abilitysystemcomponent) (break `GameplayAbilityActorInfo` (`self.GetActorInfo`)))
  (if (>= (`.ReturnValue` (`AbilitySystemBlueprintLibrary.GetFloatAttributeFromAbilitySystemComponent` _returnvalue_abilitysystemcomponent (struct :`AttributeName` "Stamina" :`Attribute` "/Script/KingdomFalls.GASAttributeSet:Stamina"))) (`.ReturnValue` (`AbilitySystemBlueprintLibrary.GetFloatAttributeFromAbilitySystemComponent` _returnvalue_abilitysystemcomponent (struct :`AttributeName` "MaxStamina" :`Attribute` "/Script/KingdomFalls.GASAttributeSet:MaxStamina"))))
    (`self.K2_EndAbility`)
    (else
      (`AbilitySystemComponent.BP_ApplyGameplayEffectToSelf` :`self` _returnvalue_abilitysystemcomponent :`GameplayEffectClass` "/Game/_KingdomFalls/Blueprints/MainCharacter/CharacterAbilities/GameplayEffects/GE_RegenStamina.GE_RegenStamina_C" :`Level` 1.0)
      (`self.RegenAgain`))))