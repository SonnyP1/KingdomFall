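; GA_ManaRegen is a Gameplay Ability that regenerates the owning character's mana after a delay.
; On activation it waits five seconds, then runs RegenManaRegen, which compares two ability system attributes, presumably current and maximum mana.
; Until the first reaches the second, it applies GE_RegenMana to itself and calls RegenMana, which repeats the check after a short WaitDelay.
; The ability ends itself once that threshold is met.
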(event `RegenMana`
  (`AbilityTask_WaitDelay.WaitDelay` 0.1
    (:`OnFinish`
      (`self.Regen_Mana_Regen` :!label _label))))

(event `self.K2_ActivateAbility`
  (`AbilityTask_WaitDelay.WaitDelay` 5.0
    (:`OnFinish`
      (goto _label))))

(fn `Regen_Mana_Regen`
  (bind (_returnvalue_owneractor _returnvalue_avataractor _returnvalue_playercontroller _returnvalue_abilitysystemcomponent) (break `GameplayAbilityActorInfo` (`self.GetActorInfo`)))
  (if (>= (`.ReturnValue` (`AbilitySystemBlueprintLibrary.GetFloatAttributeFromAbilitySystemComponent` _returnvalue_abilitysystemcomponent (struct :`AttributeName` "Mana" :`Attribute` "/Script/KingdomFalls.GASAttributeSet:Mana"))) (`.ReturnValue` (`AbilitySystemBlueprintLibrary.GetFloatAttributeFromAbilitySystemComponent` _returnvalue_abilitysystemcomponent (struct :`AttributeName` "MaxMana" :`Attribute` "/Script/KingdomFalls.GASAttributeSet:MaxMana"))))
    (`self.K2_EndAbility`)
    (else
      (`AbilitySystemComponent.BP_ApplyGameplayEffectToSelf` :`self` _returnvalue_abilitysystemcomponent :`GameplayEffectClass` "/Game/_KingdomFalls/Blueprints/MainCharacter/CharacterAbilities/GameplayEffects/Regen/GE_RegenMana.GE_RegenMana_C" :`Level` 1.0)
      (`self.RegenMana`))))