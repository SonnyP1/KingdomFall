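; Sprint gameplay ability that raises the character's MaxWalkSpeed to a running speed while draining stamina.
; On activation it caches the current max speed, then repeatedly applies GE_SprintCost every 0.1 seconds through a delay loop.
; The ability ends itself when the checked attribute hits zero, and restores the cached walking speed on end.
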(event `StaminaDrainAgain`
  (`AbilityTask_WaitDelay.WaitDelay` 0.1
    (:`OnFinish`
      (`self.StaminaDrain`))))

(event `self.K2_ActivateAbility`
  (bind (_returnvalue_owneractor _returnvalue_avataractor _returnvalue_playercontroller _returnvalue_abilitysystemcomponent _returnvalue_skeletalmeshcomponent _returnvalue_animinstance _returnvalue_movementcomponent) (break `GameplayAbilityActorInfo` (`self.GetActorInfo`)))
  (bind _ascharacter_movement_component (cast `CharacterMovementComponent` _returnvalue_movementcomponent))
  (set `self.NormalWalkingSpeed` (`MovementComponent.GetMaxSpeed` _returnvalue_movementcomponent))
  (set `CharacterMovementComponent.MaxWalkSpeed` (`self.RunningSpeed`) _ascharacter_movement_component)
  (`self.StaminaDrain`))

(event `self.K2_OnEndAbility`
  (params (bWasCancelled :type Boolean))
  (set `CharacterMovementComponent.MaxWalkSpeed` (`self.NormalWalkingSpeed`) (stale `self.K2_ActivateAbility` _ascharacter_movement_component)))

(fn `StaminaDrain`
  (bind (_returnvalue_owneractor _returnvalue_avataractor _returnvalue_playercontroller _returnvalue_abilitysystemcomponent) (break `GameplayAbilityActorInfo` (`self.GetActorInfo`)))
  (bind (_bsuccessfullyfoundattribute _returnvalue) (`AbilitySystemBlueprintLibrary.GetFloatAttributeFromAbilitySystemComponent` _returnvalue_abilitysystemcomponent (struct :`AttributeName` "Stamina" :`Attribute` "/Script/KingdomFalls.GASAttributeSet:Stamina")))
  (if _bsuccessfullyfoundattribute
    (if (<= _returnvalue 0.0)
      (`self.K2_EndAbility`)
      (else
        (`AbilitySystemComponent.BP_ApplyGameplayEffectToSelf` :`self` _returnvalue_abilitysystemcomponent :`GameplayEffectClass` "/Game/_KingdomFalls/Blueprints/MainCharacter/CharacterAbilities/GameplayEffects/Cost/GE_SprintCost.GE_SprintCost_C" :`Level` 1.0)
        (`self.StaminaDrainAgain`)))))