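; Ring of Fire Gameplay Ability: the player's magic burst that damages, stuns and knocks back nearby enemies.
; After the cost check and commit, it plays a montage on the main mesh and modular limb meshes.
; The montage notify spawns the fire effect and runs a sphere overlap that halts, damages and launches BaseAI outward, then ends the ability.
; Ending the ability attempts to activate mana regeneration.
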(event `self.K2_ActivateAbility`
  (bind (_returnvalue_owneractor _returnvalue_avataractor _returnvalue_playercontroller _returnvalue_abilitysystemcomponent _returnvalue_skeletalmeshcomponent) (break `GameplayAbilityActorInfo` (`self.GetActorInfo`)))
  (bind _returnvalue_owneractor_2 (break `GameplayAbilityActorInfo` (`self.GetActorInfo`)))
  (bind _returnvalue_owneractor_3 (break `GameplayAbilityActorInfo` (`self.GetActorInfo`)))
  (bind _returnvalue_owneractor_4 (break `GameplayAbilityActorInfo` (`self.GetActorInfo`)))
  (bind _returnvalue_owneractor_5 (break `GameplayAbilityActorInfo` (`self.GetActorInfo`)))
  (bind _returnvalue (`Actor.K2_GetActorLocation` _returnvalue_owneractor_3))
  (bind _returnvalue_2 (`self.K2_CheckAbilityCost`))
  (if _returnvalue_2
    (`self.K2_CommitAbility`)
    (bind _asbp_kingdom_falls_character (cast `/Game/_KingdomFalls/Blueprints/MainCharacter/BP_KingdomFallsCharacter` _returnvalue_owneractor))
    (for _array_element (`/Game/_KingdomFalls/Blueprints/MainCharacter/BP_KingdomFallsCharacter.LimbsAnimation` _asbp_kingdom_falls_character)
      (`|PlayMontage` _array_element "/Game/_KingdomFalls/Blueprints/MainCharacter/Assets/Animation/MagicAnimation/M_RingOfFire.M_RingOfFire"))
    (`|PlayMontage` _returnvalue_skeletalmeshcomponent "/Game/_KingdomFalls/Blueprints/MainCharacter/Assets/Animation/MagicAnimation/M_RingOfFire.M_RingOfFire"
      (:`OnInterrupted`
        (`self.K2_EndAbility`))
      (:`OnNotifyBegin`
        ;[1 1 1] DO ACTUAL WORK HERE OF THE FIRE PUSHBACK / PLAY EFFECT
        (`|SpawnActorFromClass` "/Game/_KingdomFalls/Blueprints/MainCharacter/Magic/FX/RingOfFireEffect.RingOfFireEffect_C" (`Actor.GetTransform` _returnvalue_owneractor_2) "AlwaysSpawn" "OverrideRootScale" null null)
        (set `self.Actors to Ignore` (`|MakeArray` _returnvalue_owneractor_5))
        (bind _outactors (`KismetSystemLibrary.SphereOverlapActors` (`Actor.K2_GetActorLocation` _returnvalue_owneractor_5) 500.0 (`self.Actor To Detect`) null (`self.Actors to Ignore`)))
        (for _array_element_2 _outactors
          (bind _asbase_ai (cast `/Game/_KingdomFalls/Blueprints/AI/BaseAI` _array_element_2))
          (`/Game/_KingdomFalls/Blueprints/AI/BaseAI.StopAnimationMontage` _asbase_ai)
          (`MovementComponent.StopMovementImmediately` (`Character.CharacterMovement` _asbase_ai))
          (`/Game/_KingdomFalls/Blueprints/AI/BaseAI.Took Dmg` _asbase_ai 15.0 100.0 _returnvalue_owneractor_4)
          (bind (_returnvalue_x _returnvalue_y _returnvalue_z) (`KismetMathLibrary.BreakVector` (`KismetMathLibrary.GetDirectionUnitVector` _returnvalue (`Actor.K2_GetActorLocation` _asbase_ai))))
          (bind (_returnvalue_x_2 _returnvalue_y_2) (`KismetMathLibrary.BreakVector` (* (`KismetMathLibrary.MakeVector` _returnvalue_x _returnvalue_y) (`self.KnockBackValue`))))
          (`Character.LaunchCharacter` _asbase_ai (`KismetMathLibrary.MakeVector` _returnvalue_x_2 _returnvalue_y_2 (+ _returnvalue_z 125.0)) true true))
        (`GameplayStatics.PlaySoundAtLocation` "/Game/_KingdomFalls/Blueprints/MainCharacter/Assets/Audio/sound_jump_fire.sound_jump_fire" _returnvalue (struct) 1.0 1.0 0.0 null null null)
        (`self.K2_EndAbility`)))))

(event `self.K2_OnEndAbility`
  (params (bWasCancelled :type Boolean))
  (bind (_returnvalue_owneractor _returnvalue_avataractor _returnvalue_playercontroller _returnvalue_abilitysystemcomponent _returnvalue_skeletalmeshcomponent) (break `GameplayAbilityActorInfo` (`self.GetActorInfo`)))
  (`AbilitySystemComponent.TryActivateAbilityByClass` _returnvalue_abilitysystemcomponent "/Game/_KingdomFalls/Blueprints/MainCharacter/CharacterAbilities/GameplayAbilities/MagicAbilites/GA_ManaRegen.GA_ManaRegen_C" true))