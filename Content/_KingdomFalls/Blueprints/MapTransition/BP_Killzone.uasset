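; BP_Killzone is a trigger volume that instantly kills the player character on contact.
; When a BP_KingdomFallsCharacter overlaps its Box, it activates the GA_InstaDeath gameplay ability through that character's Ability System Component, allowing remote activation.
; It also carries a PickLevelToLoad helper that looks up the current level in LevelNames to pick the following one, though nothing in this Blueprint calls it.
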(event `self.Box.OnComponentBeginOverlap`
  (params (OverlappedComponent :type "PrimitiveComponent Object Reference") (OtherActor :type "Actor Object Reference") (OtherComp :type "PrimitiveComponent Object Reference") (OtherBodyIndex :type Integer) (bFromSweep :type Boolean) (SweepResult :type "HitResult Structure (by ref)"))
  (bind _asbp_kingdom_falls_character (cast `/Game/_KingdomFalls/Blueprints/MainCharacter/BP_KingdomFallsCharacter` OtherActor))
  (`AbilitySystemComponent.TryActivateAbilityByClass` (`AbilitySystemBlueprintLibrary.GetAbilitySystemComponent` _asbp_kingdom_falls_character) "/Game/_KingdomFalls/Blueprints/MainCharacter/CharacterAbilities/GenricAbilites/GA_InstaDeath.GA_InstaDeath_C" true))

(fn `Pick Level to Load`
  (params (`Current Level` :type Name))
  (returns (`Level To Load` :type Name))
  (for (_array_element _array_index) (`self.LevelNames`)
    (if (== `Current Level` _array_element)
      (bind _result (`/Engine/EditorBlueprintResources/StandardMacros.IncrementInt` _array_index)
        (:`  `
          (return (`|GetArrayItem` (`self.LevelNames`) _result)))))))

(fn `UserConstructionScript`)