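; BaseAI is the base character for AI NPCs in Kingdom Falls, with empty events for attack, scream, flee and speed overrides.
; TookDmg plays hit feedback, applies health and stun damage gated by CanHit, and refreshes the health bar widget.
; Stun decays through a delayed recursive event, or triggers a stun montage when full.
; Zero health releases player lock-on, disables collision, enables interaction and notifies the townsperson or enemy controller.
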(event `StopAnimationMontage`
  (`self.StopAnimMontage` (`AnimInstance.GetCurrentActiveMontage` (`SkeletalMeshComponent.GetAnimInstance` (`self.Mesh`)))))

(event `ScreamAnimation`
  ;[1 1 1] Override Events
)

(event `RunningAwayAnimation`
  ;[1 1 1] Override Events
)

(event `SetSpeedToNormal`
  ;[1 1 1] Override Events
)

(event `Handle Attack 1`
  (params (CenterOverlap :type "Vector Structure") (Radius :type "Float (double-precision)") (Player :type "Object Object Reference") (Attack :type Integer))
  ;[1 1 1] Override Events
)

(event `UpdateWidgets`
  (params (Hidden :type Boolean))
  ;[1 1 1] UI
  ;;[1 1 1] UpdateWidgetsVis
  (for _array_element (`self.UI`)
    (`SceneComponent.SetHiddenInGame` _array_element Hidden false)))

(event `self.ReceiveBeginPlay`
  (bind _ui (`self.UI`))
  (`self.UpdateUI`)
  ;[1 1 1] UI
  ;;[1 1 1] Add Widgets to UI Array then sets it to hidden
  (`KismetArrayLibrary.Array_Add` _ui (`self.LockOnWidget`))
  (`KismetArrayLibrary.Array_Add` _ui (`self.HealthBarWidget`))
  (for _array_element _ui
    (`SceneComponent.SetHiddenInGame` _array_element true false))
  ;;[1 1 1] UpdateUI
  (bind _ashealth_bar (cast `/Game/_KingdomFalls/Blueprints/AI/AIUI/HealthBar` (`WidgetComponent.GetUserWidgetObject` (`self.HealthBarWidget`)) :!label _label))
  (`/Game/_KingdomFalls/Blueprints/AI/AIUI/HealthBar.UpdateHealthBar` _ashealth_bar (`self.Health`) (`self.MaxHealth`))
  (`/Game/_KingdomFalls/Blueprints/AI/AIUI/HealthBar.UpdateStunBar` _ashealth_bar (`self.Stun`) (`self.StunMax`)))

(event `UpdateUI`
  ;[1 1 1] UI
  ;;[1 1 1] UpdateUI
  (goto _label))

(event `Death`
  ;[1 1 1] Death
  (`|SpawnActorFromClass` "/Game/_KingdomFalls/Blueprints/AI/BP_DeathEffect.BP_DeathEffect_C" (`SceneComponent.K2_GetComponentToWorld` (`self.Mesh`)) "Undefined" "OverrideRootScale" null null))

(event `Took Dmg`
  (params (dmg :type "Float (double-precision)") (stunDmg :type "Float (double-precision)") (Attacker :type "Actor Object Reference"))
  (bind _returnvalue (`AIBlueprintHelperLibrary.GetAIController` self))
  (bind _returnvalue_location (`KismetMathLibrary.BreakTransform` (`self.GetTransform` self)))
  ;[1 1 1] Damage
  (`GameplayStatics.SpawnEmitterAtLocation` "/Game/FXVillesBloodVFXPack/Particles/Cascade/Real/P_Blood_Burst_Omni.P_Blood_Burst_Omni" _returnvalue_location)
  (`GameplayStatics.PlayWorldCameraShake` "/Game/_KingdomFalls/Blueprints/MainCharacter/BP_CameraHitShake.BP_CameraHitShake_C" (`self.K2_GetActorLocation` Attacker) 0.0 500.0)
  (if (`self.bCanHit`)
    (`GameplayStatics.PlaySoundAtLocation` "/Game/_KingdomFalls/Audio/limbs/attack_Sound.attack_Sound" (`self.K2_GetActorLocation`) (struct) 1.0 1.0 0.0 null null null)
    (set `self.bCanHit` false)
    (`self.PlayAnimMontage` (`self.HitReaction`))
    (set `self.isDecreasing` false)
    (bind _output_get (set `self.Health` (`KismetMathLibrary.FClamp` (- (`self.Health`) dmg) 0.0 (`self.MaxHealth`))))
    (`self.HitStun` stunDmg)
    (`self.UpdateUI`)
    (`self.StartDecraseEvent`)
    (if (<= _output_get 0.0)
      (set `self.isDead` true)
      (bind _asbp_kingdom_falls_character (cast `/Game/_KingdomFalls/Blueprints/MainCharacter/BP_KingdomFallsCharacter` Attacker)
        (:`then`
          (if (== (`KingdomFallsCharacter.lockOnTarget` _asbp_kingdom_falls_character) self)
            (`KingdomFallsCharacter.LockOnPressed` _asbp_kingdom_falls_character)))
        (:`CastFailed`
          _))
      (`PrimitiveComponent.SetCollisionEnabled` (`self.CapsuleComponent`) "NoCollision")
      (`self.StopAnimMontage` null)
      (`PrimitiveComponent.SetCollisionResponseToChannel` (`self.CapsuleComponent`) "ECC_Pawn" "ECR_Ignore")
      (set `self.isInteractable` true)
      (`self.SetDeathAnime` (`self.Mesh`))
      (bind _astown_people_ai (cast `/Game/_KingdomFalls/Blueprints/AI/Town_People/TownPeople_AI` _returnvalue)
        (:`then`
          (`/Game/_KingdomFalls/Blueprints/AI/Town_People/TownPeople_AI.Dead` _astown_people_ai))
        (:`CastFailed`
          (bind _asbp_enemy_ai (cast `/Game/_KingdomFalls/Blueprints/AI/Enemy/BP_Enemy_AI` _returnvalue)
            (:`then`
              (`/Game/_KingdomFalls/Blueprints/AI/Enemy/BP_Enemy_AI.Dead` _asbp_enemy_ai))
            (:`CastFailed`
              (`KismetSystemLibrary.PrintString` "cast faile"))))))))

(event `StartDecraseEvent`
  ;[1 1 1] Stun Mechanic
  ;;[1 1 1] StartDecreaseStun
  (`KismetSystemLibrary.Delay` 5.0)
  (set `self.isDecreasing` true)
  (`self.DecreaseStun`))

(event `DecreaseStun`
  ;[1 1 1] Stun Mechanic
  ;;[1 1 1] DecreaseStun
  (if (`self.isDecreasing`)
    (bind _output_get (set `self.Stun` (`KismetMathLibrary.FClamp` (- (`self.Stun`) (`self.StunDecreasePerSec`)) 0.0 (`self.StunMax`))))
    (`self.UpdateUI`)
    (if (== _output_get 0.0)
      (set `self.isDecreasing` false)
      (else
        (`KismetSystemLibrary.Delay` 0.2)
        (`self.DecreaseStun`)))))

(event `HitStun`
  (params (StunDmg :type "Float (double-precision)"))
  (bind _hitstunmontage (`self.HitStunMontage`))
  ;[1 1 1] Stun Mechanic
  ;;[1 1 1] HitStun
  (bind _output_get (set `self.Stun` (+ (`self.Stun`) StunDmg)))
  (`self.UpdateUI`)
  (if (>= _output_get (`self.StunMax`))
    (if (!= (`self.GetCurrentMontage`) _hitstunmontage)
      (`|PlayMontage` (`self.Mesh`) _hitstunmontage
        (:`OnCompleted`
          (set `self.Stun` 0.0)
          (`self.UpdateUI`))))))

(fn `EndHitstop`
  (params (actor :type "Actor Object Reference"))
  (`KismetSystemLibrary.PrintString` "Resume")
  (set `self.CustomTimeDilation` 1.0))

(fn `SetDeathAnime`
  (params (mesh :type "SkeletalMeshComponent Object Reference"))
  (returns (AI :type "SkeletalMeshComponent Object Reference"))
  (bind _asanime_bp_noblewomen (cast `/Game/_KingdomFalls/Blueprints/AI/Town_People/Noblewomen/Animation/AnimeBP_Noblewomen` (`SkeletalMeshComponent.GetAnimInstance` mesh)))
  (set `/Game/_KingdomFalls/Blueprints/AI/Town_People/Noblewomen/Animation/AnimeBP_Noblewomen.isDead` true _asanime_bp_noblewomen)
  (return mesh))

(fn `StartHitstop`
  (params (duration :type "Float (double-precision)"))
  (set `self.CustomTimeDilation` 0.0)
  (`KismetSystemLibrary.K2_SetTimer` null "EndHitstop" duration))

(fn `UserConstructionScript`)